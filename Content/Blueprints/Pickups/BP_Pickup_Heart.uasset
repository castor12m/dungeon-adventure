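; BP_Pickup_Heart is a pickup that restores health to the hero who collects it.
; It overrides HandlePickup, calls the parent implementation, then calls GetHealed on the hero with its HealAmount.
; Collection logic is not defined here; BeginPlay, overlap and Tick are disabled stubs, and the construction script only calls the parent.
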(event EventBeginPlay
  (|CallParentFunction) ; This node is disabled and will not be called.\nDrag off pins to build functionality.
)

(event Collision|EventActorBeginOverlap
  (params (OtherActor :type Actor%20Object%20Reference))
  (|CallParentFunction OtherActor) ; This node is disabled and will not be called.\nDrag off pins to build functionality.
)

(event EventTick
  (params (DeltaSeconds :type Float%20%28single-precision%29))
  (|CallParentFunction DeltaSeconds) ; This node is disabled and will not be called.\nDrag off pins to build functionality.
)

(event EventHandlePickup
  (params (Hero :type BP%20Hero%20Object%20Reference))
  (|CallParentFunction Hero)
  (Default|GetHealed Hero (Variables|Default|GetHealAmount)))

(fn ConstructionScript
  (|CallParentFunction))